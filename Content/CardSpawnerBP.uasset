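; Card spawner for an Empire-versus-Rebellion card game that builds both players' decks.
; BeginPlay caches the GameManager, loads all cards and resets their row to Player One's deck, since changes carry into repeated plays.
; FactionChosen spawns the player's chosen faction, moves the opposing faction to Player Two's deck and spawns it, then passes all card actors to GameManager.AllCardsSpawned.
; Disconnected prototype SpawnCard calls remain and never run.
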(event `self.ReceiveBeginPlay`
  (bind _asgame_manager (cast `/Game/GameManager` (`GameplayStatics.GetGameMode`)))
  (bind _output_get (set `self.Game Manager Ref` _asgame_manager))
  (bind _returnvalue (`self.LoadAllCards`)) ; Should be the first function called when the game begins
  (bind _output_get_2 (set `self.Cards` _returnvalue))
  (if (`KismetArrayLibrary.Array_IsEmpty` _output_get_2)
    (`KismetSystemLibrary.LogString` "Ruh roh Raggy")
    (else
      (`KismetSystemLibrary.LogString` "We good")
      (for _array_element _output_get_2
        (set `Card.CardRow` "PlayerOneDeck" _array_element) ; Set all cards to Player One Deck at start of game, for repeated plays
      )
      (`KismetSystemLibrary.LogString` "Card Row Reset"))))

(event `FactionChosen`
  (bind _cards (`self.Cards`))
  (bind _cardsactors (`self.CardsActors`))
  (bind _cardsactors_2 (`self.CardsActors`))
  (switch `ECardFaction` (`/Game/GameManager.PlayerOneChosenFaction` (stale `self.ReceiveBeginPlay` _output_get))
    (:`Empire`
      (`KismetSystemLibrary.LogString` "Player chose \"Empire\"")
      ; Spawn the Player's chosen Deck
      (bind _returnvalue (`self.SpawnRow` "Empire" "PlayerOneDeck"))
      (`KismetArrayLibrary.Array_Append` _cardsactors _returnvalue)
      (`KismetSystemLibrary.LogString` "Player Deck spawned")
      (for _array_element _cards
        (switch `ECardFaction` (`Card.CardFaction` _array_element)
          (:`Rebellion`
            (bind _output_get (set `Card.CardRow` "PlayerTwoDeck" _array_element))
            (`KismetSystemLibrary.LogString` (`KismetStringLibrary.Concat_StrStr` (`KismetStringLibrary.Concat_StrStr` "Card Name: " (`Card.CardName` _array_element)) (`KismetStringLibrary.Concat_StrStr` " Card Faction: " (`|GetEnumeratorNameAsString` _output_get)))))))
      (bind _returnvalue_2 (`self.SpawnRow` "Rebellion" _output_get))
      (`KismetArrayLibrary.Array_Append` _cardsactors_2 _returnvalue_2)
      (`/Game/GameManager.AllCardsSpawned` (`self.Game Manager Ref`) _cardsactors_2 :!label _label))
    (:`Rebellion`
      (`KismetSystemLibrary.LogString` "Player chose \"Rebellion\"")
      (bind _returnvalue_3 (`self.SpawnRow` "Rebellion" "PlayerOneDeck"))
      (`KismetArrayLibrary.Array_Append` _cardsactors _returnvalue_3)
      (`KismetSystemLibrary.LogString` "Player Deck spawned")
      (for _array_element_2 _cards
        (switch `ECardFaction` (`Card.CardFaction` _array_element_2)
          (:`Empire`
            (bind _output_get_2 (set `Card.CardRow` "PlayerTwoDeck" _array_element_2))
            (`KismetSystemLibrary.LogString` (`KismetStringLibrary.Concat_StrStr` (`KismetStringLibrary.Concat_StrStr` "Card Name: " (`Card.CardName` _array_element_2)) (`KismetStringLibrary.Concat_StrStr` " Card Faction: " (`|GetEnumeratorNameAsString` _output_get_2)))))))
      (bind _returnvalue_4 (`self.SpawnRow` "Empire" "PlayerTwoDeck"))
      (`KismetArrayLibrary.Array_Append` _cardsactors_2 _returnvalue_4)
      (goto _label))
    (:`Neutral`
      (`KismetSystemLibrary.LogString` "NOT POSSIBLE"))))

(fn `UserConstructionScript`)